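; Spawner actor that scatters a batch of large rock meshes around itself at BeginPlay, apparently as distant scenery.
; A loop spawns plain StaticMeshActors on a wide spherical shell around the actor, using random unit vectors at a fixed radius.
; Each gets a random rotation and per-axis scale, is assigned SM_Rock and has collision disabled.
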(event `self.ReceiveBeginPlay`
  (for _ (range 31)
    (bind _returnvalue (`|SpawnActorFromClass` "/Script/Engine.StaticMeshActor" (`KismetMathLibrary.MakeTransform` (+ (`self.K2_GetActorLocation`) (* (`KismetMathLibrary.RandomUnitVector`) (100000.0 100000.0 100000.0))) (`KismetMathLibrary.RandomRotator` true) (`KismetMathLibrary.MakeVector` (`KismetMathLibrary.RandomFloatInRange` 20.0 100.0) (`KismetMathLibrary.RandomFloatInRange` 20.0 100.0) (`KismetMathLibrary.RandomFloatInRange` 20.0 100.0))) "AlwaysSpawn" "OverrideRootScale" null null))
    (bind _staticmeshcomponent (`StaticMeshActor.StaticMeshComponent` _returnvalue))
    (`StaticMeshComponent.SetStaticMesh` _staticmeshcomponent "/Game/StarterContent/Props/SM_Rock.SM_Rock")
    (`PrimitiveComponent.SetCollisionEnabled` _staticmeshcomponent "NoCollision")))

(fn `UserConstructionScript`)